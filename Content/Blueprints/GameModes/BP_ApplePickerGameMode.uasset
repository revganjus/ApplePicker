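; Game mode for an apple-picking game that handles apple hits and timed level progression.
; On begin play it caches the game state, shows the HUD and starts a looping timer that levels up both the apple tree and the game state.
; An apple hitting a basket adds its score through the game state, while hitting anything else opens a level by object reference.
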(event EventBeginPlay
  (bind _asbp_apple_picker_game_state (Utilities|Casting|CastToBP_ApplePickerGameState (Game|GetGameState)))
  (Variables|Service|SetApplePickerGameState _asbp_apple_picker_game_state)
  (Utilities|Time|SetTimerbyFunctionName 0 "UpLevel" (Variables|Config|GetNextLevelInterval) true)
  (bind _returnvalue (UserInterface|CreateWidget "/Game/Blueprints/UI/WBP_HUD.WBP_HUD_C" (Game|GetPlayerController 0)))
  (UserInterface|Viewport|AddtoViewport _returnvalue 0))

(fn ConstructionScript)

(fn OnAppleHit
  (params (HitObject :type Object%20Object%20Reference) (AppleScore :type Integer))
  (Utilities|Casting|CastToBP_BasketBase HitObject
    (:then
      (Default|OnAppleCaught (Variables|Service|GetApplePickerGameState) AppleScore))
    (:CastFailed
      (Game|OpenLevel(byObjectReference) "/Game/Maps/_Scene_0._Scene_0"))))

(fn UpLevel
  (bind _returnvalue (Actor|GetActorOfClass "/Game/Blueprints/Actors/BP_AppleTree.BP_AppleTree_C"))
  (Default|UpLevel _returnvalue)
  (Default|OnLevelUp (Variables|Service|GetApplePickerGameState)))