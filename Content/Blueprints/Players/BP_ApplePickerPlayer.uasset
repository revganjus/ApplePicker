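; BP_ApplePickerPlayer is the apple-picker player, controlling a row of baskets that follows the mouse horizontally.
; On BeginPlay it spawns randomly round or square baskets, evenly spaced around an offset from BP_AppleTree's ground-projected drop point, and maps each to an X offset.
; Each Tick it deprojects the cursor to a fixed-distance world point and sets each basket's X from it plus that offset, keeping Y and Z.
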(event EventBeginPlay
  (bind _location (Service|GetCentalBasketLocation))
  (Service|SpawnBaskets _location))

(event EventTick
  (params (DeltaSeconds :type Float%20%28single-precision%29))
  (bind _returnvalue (Game|GetPlayerController 0))
  (bind _bastettoxoffset (Variables|Service|GetBastetToXOffset))
  (bind (_worldlocation _worlddirection) (Game|Player|ConvertMouseLocationToWorldSpace _returnvalue))
  (bind _keys (Utilities|Map|Keys _bastettoxoffset))
  (for _array_element _keys
    (Transformation|SetActorLocation _array_element (Math|Vector|MakeVector (+ (.Value (Utilities|Map|Find _bastettoxoffset _array_element)) (.x (+ _worldlocation (* _worlddirection 1e+03)))) (.y (Transformation|GetActorLocation _array_element)) (.z (Transformation|GetActorLocation _array_element))) false false)))

(fn ConstructionScript)

(fn GetCentalBasketLocation
  (bind _returnvalue (Actor|GetActorOfClass "/Game/Blueprints/Actors/BP_AppleTree.BP_AppleTree_C"))
  (bind _droplocation (Default|GetAppleDropLocation _returnvalue))
  (return (+ (Math|Vector|MakeVector (.x _droplocation) (.y _droplocation) 0.0) (Variables|Config|GetBasketOffset))))

(fn SpawnBaskets
  (params (CentralLocation :type Vector))
  (bind (_x _y _z) (Math|Vector|BreakVector CentralLocation))
  (LocalVariables|SetStartLocation (Math|Vector|MakeVector (- _x (/ (* (- (Variables|Config|GetBasketsCount) 1) (Variables|Config|GetBasketSpacing)) 2.0)) _y _z))
  (for _index (range 0 (- (Variables|Config|GetBasketsCount) 1))
    (bind _newparam (Service|GetBasketClass))
    (bind _returnvalue (Game|SpawnActorfromClass _newparam (Math|Conversions|ToTransform(Vector) (LocalVariables|GetStartLocation)) "Undefined" 0 0))
    (Utilities|Map|Add (Variables|Service|GetBastetToXOffset) _returnvalue (- (.x CentralLocation) (.X (Math|Vector|BreakVector (LocalVariables|GetStartLocation)))))
    (LocalVariables|SetStartLocation (Math|Vector|MakeVector (+ (.x (LocalVariables|GetStartLocation)) (Variables|Config|GetBasketSpacing)) (.y (LocalVariables|GetStartLocation)) (.z (LocalVariables|GetStartLocation))))))

(fn GetBasketClass
  (if (Math|Random|RandomBool)
    (return "/Game/Blueprints/Actors/Basket/BP_RoundBasket.BP_RoundBasket_C")
    (else
      (return "/Game/Blueprints/Actors/Basket/BP_SquareBasket.BP_SquareBasket_C"))))