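; Apple tree actor that slides back and forth along X around its start position, periodically dropping apples for an apple-catching style game.
; Two looping timers drive it: one spawns a common or rare apple by weighted chance below an offset, the other updates movement.
; Movement scales speed by the timer's elapsed time, reversing at the edges or at random.
; UpLevel raises speed by a fixed increment derived from the initial speed.
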(event EventBeginPlay
  (bind _returnvalue (Transformation|GetActorLocation))
  (Variables|Service|SetLeftEdge (- (.x _returnvalue) (Variables|Config|GetHalfDistance)))
  (Variables|Service|SetRightEdge (+ (.x _returnvalue) (Variables|Config|GetHalfDistance)))
  (Variables|Service|SetUpLevelMoveSpeedDelta (Math|Float|Absolute(Float) (* (Variables|Config|GetMoveSpeed) (Variables|Config|GetUpLevelMoveSpeedCoefficient))))
  (Service|SetupTimers))

(fn ConstructionScript)

(fn DropApple
  (bind _droplocation (CallFunction|GetAppleDropLocation))
  (bind _appleclass (Service|GetAppleClass))
  (Game|SpawnActorfromClass _appleclass (Math|Conversions|ToTransform(Vector) _droplocation) "AdjustIfPossibleButAlwaysSpawn" 0 0))

(fn UpdateMovement
  (bind _returnvalue (Transformation|GetActorLocation))
  (Transformation|SetActorLocation (Math|Vector|MakeVector (+ (* (Variables|Config|GetMoveSpeed) (Class|KismetSystemLibrary|GetTimerElapsedTimeHandle (Variables|Service|GetMovementTimerHandle))) (.x _returnvalue)) (.y _returnvalue) (.z _returnvalue)) false false)
  (Service|TryChangeDirection))

(fn TryChangeDirection
  (LocalVariables|SetCurrentX (.x (Transformation|GetActorLocation)))
  (if (< (LocalVariables|GetCurrentX) (Variables|Service|GetLeftEdge))
    (Variables|Config|SetMoveSpeed (Math|Float|Absolute(Float) (Variables|Config|GetMoveSpeed)))
    (elif (> (LocalVariables|GetCurrentX) (Variables|Service|GetRightEdge))
      (bind _result (Math|Float|NegateFloat (Math|Float|Absolute(Float) (Variables|Config|GetMoveSpeed)))
        (:%20%20
          (Variables|Config|SetMoveSpeed _result)))
      (elif (Math|Random|RandomBoolwithWeight (Variables|Config|GetChangeDirectionChance))
        (bind _result_2 (Math|Float|NegateFloat (Variables|Config|GetMoveSpeed))
          (:%20%20
            (Variables|Config|SetMoveSpeed _result_2)))))))

(fn UpLevel
  (Variables|Config|SetMoveSpeed (+ (Math|Float|Absolute(Float) (Variables|Config|GetMoveSpeed)) (Variables|Service|GetUpLevelMoveSpeedDelta))))

(fn GetAppleDropLocation
  (return (- (Transformation|GetActorLocation) (Variables|Config|GetAppleDropOffset))))

(fn SetupTimers
  (Utilities|Time|ClearandInvalidateTimerbyHandle (Variables|Service|GetDropTimerHandle))
  (bind _returnvalue (Utilities|Time|SetTimerbyFunctionName 0 "DropApple" (Variables|Config|GetAppleDropsInterval) true))
  (Variables|Service|SetDropTimerHandle _returnvalue)
  (Utilities|Time|ClearandInvalidateTimerbyHandle (Variables|Service|GetMovementTimerHandle))
  (bind _returnvalue_2 (Utilities|Time|SetTimerbyFunctionName 0 "UpdateMovement" (Variables|Config|GetUpdateMovementInterval) true))
  (Variables|Service|SetMovementTimerHandle _returnvalue_2))

(fn GetAppleClass
  (if (Math|Random|RandomBoolwithWeight (Variables|Config|GetRareAppleChance))
    (return "/Game/Blueprints/Actors/Apple/BP_RareApple.BP_RareApple_C")
    (else
      (return "/Game/Blueprints/Actors/Apple/BP_Apple.BP_Apple_C"))))