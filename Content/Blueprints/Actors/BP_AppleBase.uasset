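; Base apple actor for an apple picker game, carrying a score and material determined by its AppleType.
; The construction script uses the enum's name as the row key into DT_Apples to set Score and the Apple component's material.
; On BeginPlay it caches the game mode; on Hit it passes the hit object and Score to the game mode's OnAppleHit, then destroys itself.
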(event EventBeginPlay
  (bind _asbp_apple_picker_game_mode (Utilities|Casting|CastToBP_ApplePickerGameMode (Game|GetGameMode)))
  (Variables|Service|SetApplePickerGameMode _asbp_apple_picker_game_mode))

(event Collision|EventHit
  (params (MyComp :type Primitive%20Component%20Object%20Reference) (Other :type Actor%20Object%20Reference) (OtherComp :type Primitive%20Component%20Object%20Reference) (bSelfMoved :type Boolean) (HitLocation :type Vector :default "0, 0, 0") (HitNormal :type Vector :default "0, 0, 0") (NormalImpulse :type Vector :default "0, 0, 0") (Hit :type Hit%20Result%20Structure%20%28by%20ref%29))
  (Default|OnAppleHit (Variables|Service|GetApplePickerGameMode) Other (Variables|Service|GetScore))
  (Actor|DestroyActor))

(fn ConstructionScript
  (bind _returnvalue (Utilities|GetDataTableRow "/Game/Blueprints/DT_Apples.DT_Apples" (Utilities|String|StringToName (Utilities|String|EnumtoString (Variables|Default|GetAppleType))))
    (:then
      (Variables|Service|SetScore (.Score (Utilities|Struct|BreakSAppleInfo _returnvalue)))
      (Rendering|Material|SetMaterial (Variables|Default|GetApple) 0 (.Material (Utilities|Struct|BreakSAppleInfo _returnvalue))))))